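; BP_TestCrate is a pickup crate that reacts when a player-controlled pawn enters its Sphere1 overlap volume.
; On overlap it plays a pirate voice sound at its location and adds a PickUpDia widget to the viewport.
; It then reports the pickup to BP_ProceduralManager via SoulCollected and calls DestroyCrates on its linked CrateLink reference.
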(event OnComponentBeginOverlap(Sphere1)
  (params (OverlappedComponent :type Primitive%20Component%20Object%20Reference) (OtherActor :type Actor%20Object%20Reference) (OtherComp :type Primitive%20Component%20Object%20Reference) (OtherBodyIndex :type Integer) (bFromSweep :type Boolean) (SweepResult :type Hit%20Result%20Structure%20%28by%20ref%29))
  (bind _aspawn (Utilities|Casting|CastToPawn OtherActor))
  (if (Pawn|IsPlayerControlled _aspawn)
    (Audio|PlaySoundatLocation "/Game/Sound/476324__jd-brick-productions__pirate-arr-1.476324__jd-brick-productions__pirate-arr-1" (Transformation|GetActorLocation) "0, 0, 0" 1.0 1.0 0.0 0 0 0)
    (bind _returnvalue (UserInterface|CreateWidget "/Game/UI/PickUpDia.PickUpDia_C"))
    (UserInterface|Viewport|AddtoViewport _returnvalue 0)
    (bind _returnvalue_2 (Actor|GetActorOfClass "/Game/Blueprints/BP_ProceduralManager.BP_ProceduralManager_C"))
    (Class|ProceduralManager|SoulCollected _returnvalue_2)
    (Class|CrateLink|DestroyCrates (Variables|Default|GetCrateLink))))

(fn ConstructionScript)